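; BP_RestartTrigger is a level trigger that restarts the current level for the player, with camera fades.
; BeginPlay fades the camera in from opaque, and the Box overlap event caches the current level name.
; The player check runs on Tick against the overlap's OtherActor, rather than inside the overlap event.
; On a match it fades the camera out, waits for the fade, then reopens the cached level by name.
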(event OnComponentBeginOverlap(Box)
  (params (OverlappedComponent :type Primitive%20Component%20Object%20Reference) (OtherActor :type Actor%20Object%20Reference) (OtherComp :type Primitive%20Component%20Object%20Reference) (OtherBodyIndex :type Integer) (bFromSweep :type Boolean) (SweepResult :type Hit%20Result%20Structure%20%28by%20ref%29))
  (bind _returnvalue (Game|GetCurrentLevelName true)))

(event EventTick
  (params (DeltaSeconds :type Float%20%28single-precision%29))
  (if (== (stale OnComponentBeginOverlap(Box) OtherActor) (Game|Player|GetPlayerPawn 0))
    (CameraFades|StartCameraFade :self (Game|GetPlayerCameraManager 0) :ToAlpha 1.0 :Duration 1.0)
    (Utilities|FlowControl|Delay (Math|Float|MakeLiteralFloat 1.0))
    (Game|OpenLevel(byName) (Utilities|String|StringToName (stale OnComponentBeginOverlap(Box) _returnvalue)))))

(event EventBeginPlay
  (CameraFades|StartCameraFade :self (Game|GetPlayerCameraManager 0) :FromAlpha 1.0 :ToAlpha 0.0 :Duration 1.0))

(fn ConstructionScript)